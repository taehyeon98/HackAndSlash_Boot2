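; BP_SkillBase is a skill actor for the hack-and-slash game that damages monsters it overlaps and removes itself after a set lifetime.
; On BeginPlay it looks up its SkillRowName in DT_Skill and starts a timer from that row's LifeTime, which calls LifeTimeOver to destroy it.
; Overlapping a BP_MonsterBase applies hardcoded damage, independent of the table, credited to the skill's owner and its instigator controller.
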(event EventBeginPlay
  (bind _returnvalue (Utilities|GetDataTableRow "/Game/HackAndSlash/Skills/DT_Skill.DT_Skill" (Variables|Default|GetSkillRowName))
    (:then
      (Utilities|Time|SetTimerbyFunctionName 0 "LifeTimeOver" (.LifeTime (Utilities|Struct|BreakST_Skill _returnvalue))))))

(event Collision|EventActorBeginOverlap
  (params (OtherActor :type Actor%20Object%20Reference))
  (bind _returnvalue (Components|GetOwner))
  (bind _asbp_monster_base (Utilities|Casting|CastToBP_MonsterBase OtherActor))
  (Game|Damage|ApplyDamage _asbp_monster_base 1e+02 (Game|GetInstigatorController _returnvalue) _returnvalue))

(fn ConstructionScript)

(fn LifeTimeOver
  (Actor|DestroyActor))