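; Game mode for the hack-and-slash game that drives match phases stored in BP_HSGameState.
; On BeginPlay it binds to the game state's change dispatcher and enters Ready, then Tick switches to Play once total time reaches five seconds.
; State changes set game-only input with a hidden cursor, except End, which pauses and shows the cursor with UI-only input.
; UpdatePlay can end the game at zero HP but is not called here.
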(event EventBeginPlay
  (bind _asbp_hsgame_state (Utilities|Casting|CastToBP_HSGameState (Game|GetGameState)))
  (EventDispatchers|BindEventtoEventDispatcherChangeGameState _asbp_hsgame_state (EventDispatchers|CreateEvent :!event EventChangeGameState))
  (Default|ChangeGameState _asbp_hsgame_state "NewEnumerator1"))

(event EventTick
  (params (DeltaSeconds :type Float%20%28single-precision%29))
  (bind _asbp_hsgame_state (Utilities|Casting|CastToBP_HSGameState (Game|GetGameState)))
  (switch Utilities|FlowControl|Switch|SwitchonEN_GameState (Variables|/Game/HackAndSlash/GameMode/BP_HSGameState.BP_HSGameState_C|GetHSGameState _asbp_hsgame_state)
    (:NewEnumerator1
      (CallFunction|UpdateReady (Variables|/Game/HackAndSlash/GameMode/BP_HSGameState.BP_HSGameState_C|GetTotalDeltaTime _asbp_hsgame_state) _asbp_hsgame_state))))

(fn ConstructionScript)

(fn UpdatePlay
  (params (CurHp :type Float%20%28double-precision%29) (GameState :type BP%20HS%20Game%20State%20Object%20Reference))
  (if (<= CurHp 0.0)
    (Default|ChangeGameState GameState "NewEnumerator3")))

(fn UpdateReady
  (params (TotalTime :type Float%20%28double-precision%29) (GameState :type BP%20HS%20Game%20State%20Object%20Reference))
  (if (>= TotalTime 5.0)
    (Default|ChangeGameState GameState "NewEnumerator2")))

(fn UpdateEnd
  (params (IsDeath :type Boolean))
  (if IsDeath
    _))

(fn EventChangeGameState
  (params (HSGameState :type EN_GameState%20Enum :default "NewEnumerator0"))
  (bind _returnvalue (Game|GetPlayerController 0))
  (bind _returnvalue_2 (Game|GetPlayerController 0))
  (switch Utilities|FlowControl|Switch|SwitchonEN_GameState HSGameState
    (:NewEnumerator0
      (Input|SetInputModeGameOnly _returnvalue_2 false :!label _label)
      (Variables|/Script/Engine.PlayerController|SetbShowMouseCursor _returnvalue_2 false))
    (:NewEnumerator1
      (goto _label))
    (:NewEnumerator2
      (goto _label))
    (:NewEnumerator3
      (Game|SetGamePaused true)
      (Input|SetInputModeUIOnly _returnvalue 0 "DoNotLock" false)
      (Variables|/Script/Engine.PlayerController|SetbShowMouseCursor _returnvalue true))))