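; BP_HSGameState is the game state Blueprint for the HackAndSlash game, holding the current HSGameState and the time spent in it.
; Tick adds delta seconds to a running TotalDeltaTime.
; ChangeGameState acts only when the state differs, resetting the timer, storing and printing the new state, then broadcasting it through the ChangeGameState event dispatcher.
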(event EventTick
  (params (DeltaSeconds :type Float%20%28single-precision%29))
  (Variables|Default|SetTotalDeltaTime (+ DeltaSeconds (Variables|Default|GetTotalDeltaTime))))

(fn ConstructionScript)

(fn ChangeGameState
  (params (HSGameState :type EN_GameState%20Enum :default "NewEnumerator0"))
  (if (Utilities|Enum|NotEqual(Enum) HSGameState (Variables|Default|GetHSGameState))
    (Variables|Default|SetTotalDeltaTime 0.0)
    (bind _output_get (Variables|Default|SetHSGameState HSGameState))
    (Development|PrintString (Utilities|String|Append " GameState : " (Utilities|String|EnumtoString _output_get)))
    (Default|CallEventDispatcherChangeGameState _output_get)))